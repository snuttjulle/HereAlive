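; Watering can actor that waters the level's Flower whenever the game mode's ChatManager has a queued watering request and the flower is alive.
; A Tick-driven state machine cycles Hidden, In, Watering and Out, scaling in with an elastic math expression and out with a float curve.
; A timer matched to the watering animation waters the flower, then either repeats for the next queued request or scales away.
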(event Custom|ChatManagerWasCreated
  (Variables|Default|SetChatManager (stale EventBeginPlay _chatmanager)))

(event EventTick
  (params (DeltaSeconds :type Float%20%28single-precision%29))
  (switch Utilities|FlowControl|Switch|SwitchonWateringCanState (Variables|Default|GetCurrentState)
    (:NewEnumerator0
      ;[1 1 1] Spawn Animation
      (bind _output_get (Variables|Default|SetElapsedTime (+ DeltaSeconds (Variables|Default|GetElapsedTime)) :!label _label))
      (if (< (Variables|Default|GetElapsedTime) (Variables|Default|GetSpawnTime))
        (if (Utilities|Enum|Equal(Enum) (Variables|Default|GetCurrentState) "NewEnumerator0")
          (Transformation|SetActorScale3D (Math|Conversions|ToVector(Float) (|((((sin(((value*PI)*(0.200000+(((2.500000*value)*value)*value)))))*(pow((1.000000-value),2.200000)))+value)*(1.000000+(1.200000*(1.000000-value)))) (Math|Float|Clamp(Float) (/ _output_get (Variables|Default|GetSpawnTime))) (Math|Trig|GetPI))))
          (else
            (Transformation|SetActorScale3D (Math|Conversions|ToVector(Float) (Math|Curves|GetFloatValue (Variables|Default|GetOutAnimationCurve) (Math|Float|Clamp(Float) (/ _output_get (Variables|Default|GetSpawnTime))))))))
        (else
          (switch Utilities|FlowControl|Switch|SwitchonWateringCanState (Variables|Default|GetCurrentState)
            (:NewEnumerator0
              (CallFunction|SetWateringCanState "NewEnumerator1"))
            (:NewEnumerator2
              (CallFunction|SetWateringCanState "NewEnumerator3"))))))
    (:NewEnumerator2
      (goto _label))
    (:NewEnumerator3
      (bind _newrequestishandled (CallFunction|TryandPopPendingWateringRequest))
      (if _newrequestishandled
        (CallFunction|SetWateringCanState "NewEnumerator0")))))

(event EventBeginPlay
  (Transformation|SetActorScale3D "0, 0, 0")
  (CallFunction|SetWateringCanState "NewEnumerator3")
  (bind _outactors (Actor|GetAllActorsOfClass "/Game/KeepItAlive/Blueprints/Flower.Flower_C"))
  (Variables|Default|SetFlower (Utilities|Array|Get(acopy) _outactors))
  (bind _asflower_game_mode (Utilities|Casting|CastToFlowerGameMode (Game|GetGameMode)))
  (bind _chatmanager (Variables|/Game/KeepItAlive/Blueprints/FlowerGameMode.FlowerGameMode_C|GetChatManager _asflower_game_mode)
    (:then
      (Variables|Default|SetChatManager _chatmanager))
    (:else
      (EventDispatchers|BindEventtoOnChatManagerCreated _asflower_game_mode (delegate Custom|ChatManagerWasCreated)))))

(fn ConstructionScript)

(fn SetWateringCanState
  (params (NewState :type WateringCanState%20Enum :default "NewEnumerator0"))
  (Utilities|FlowControl|Sequence
    (:then_0
      (switch Utilities|FlowControl|Switch|SwitchonWateringCanState NewState
        (:NewEnumerator0
          ;[1 1 1] In
          (Variables|Default|SetElapsedTime 0.0)
          (Audio|PlaySoundatLocation "/Game/KeepItAlive/Audio/BucketEquip.BucketEquip" (Transformation|GetActorLocation) "0, 0, 0" 1.0 1.0 0.0 0 0 0))
        (:NewEnumerator1
          ;[1 1 1] Watering
          (Components|Animation|PlayAnimation (Variables|Default|GetWateringCan) "/Game/KeepItAlive/WateringCan/WateringCan_Anim.WateringCan_Anim" false)
          (bind _returnvalue (Utilities|Time|SetTimerbyEvent (EventDispatchers|CreateEvent :!event OnAnimationFinished) 6.3))
          (Variables|Default|SetTimerHandle _returnvalue))
        (:NewEnumerator2
          ;[1 1 1] Out
          (Variables|Default|SetElapsedTime 0.0)
          (Audio|PlaySoundatLocation "/Game/KeepItAlive/Audio/BucketEquip.BucketEquip" (Transformation|GetActorLocation) "0, 0, 0" 1.0 1.0 0.0 0 0 0))
        (:NewEnumerator3
          ;[1 1 1] Hidden
          (Transformation|SetActorScale3D "0, 0, 0")
          (Variables|Default|SetElapsedTime 0.0))))
    (:then_1
      (Variables|Default|SetCurrentState NewState))))

(fn OnAnimationFinished
  (Class|KIAFlower|WaterFlower (Variables|Default|GetFlower))
  (bind _newrequestishandled (CallFunction|TryandPopPendingWateringRequest))
  (if _newrequestishandled
    (CallFunction|SetWateringCanState "NewEnumerator1")
    (else
      (CallFunction|SetWateringCanState "NewEnumerator2"))))

(fn TryandPopPendingWateringRequest
  (if (Class|KIAFlower|IsAlive (Variables|Default|GetFlower))
    (bind _chatmanager (Variables|Default|GetChatManager)
      (:then
        (if (Class|KIAChatManager|HasPendingWateringRequests _chatmanager)
          (bind _returnvalue (Class|KIAChatManager|PopWateringRequestQueue _chatmanager))
          (if (Utilities|Enum|NotEqual(Enum) _returnvalue "")
            _
            (else
              _))
          (return true)
          (else
            (return false))))
      (:else))))