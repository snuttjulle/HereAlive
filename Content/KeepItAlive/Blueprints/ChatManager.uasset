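; ChatManager connects the game to Twitch chat through the TwitchPlay plugin, showing messages as floating text and handling a "water" chat command.
; On BeginPlay it caches the WateringCan, authenticates with credentials from a data table, then binds message and command callbacks.
; Messages go to a lazily found FloatingTextSpawner, dropping any that triggers the lookup.
; Water commands forward to ExecuteWaterCommand, with the K key simulating one for debugging.
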(event `self.ReceiveBeginPlay`
  (bind _mtwitchplaycomponent (`self.mTwitchPlayComponent`))
  (bind _outactors (`GameplayStatics.GetAllActorsOfClass` "/Game/KeepItAlive/Blueprints/WateringCan.WateringCan_C"))
  (set `self.WateringCan` (`|GetArrayItem` _outactors))
  ;[1 1 1] Setup the TwitchPlay plugin
  (bind _returnvalue (`|GetDataTableRow` "/Game/KeepItAlive/Authentication/AuthDataTable.AuthDataTable" "HereAlive")
    (:`then`
      (bind (_oauthtoken _username _channelname) (break `TwitchAuthenticationData` _returnvalue))
      (`TwitchIRCComponent.SetUserInfo` (`self.mTwitchPlayComponent`) _oauthtoken _username _channelname)
      (bind (__out_error _returnvalue_2) (`TwitchIRCComponent.Connect` (`self.mTwitchPlayComponent`)))
      (if _returnvalue_2
        (bind (__out_error_2 _returnvalue_3) (`TwitchIRCComponent.AuthenticateTwitchIRC` (`self.mTwitchPlayComponent`)))
        (if _returnvalue_3
          (add `TwitchIRCComponent.OnMessageReceived` (`self.mTwitchPlayComponent`) (`|CreateDelegate` :!event `OnMessageReceived`))
          (`TwitchPlayComponent.SetupEncapsulationChars` (`self.mTwitchPlayComponent`) (`TwitchPlayComponent.command_encapsulation_char_` _mtwitchplaycomponent) (`TwitchPlayComponent.options_encapsulation_char_` _mtwitchplaycomponent))
          (bind (__out_result _returnvalue_4) (`TwitchPlayComponent.RegisterCommand` (`self.mTwitchPlayComponent`) "water" (`|CreateDelegate` :!event `OnWaterCmd`)))
          (if _returnvalue_4
            _))))))

(event `Key|K`
  (params (Key :type "Key Structure"))
  (:`Pressed`
    (`self.OnWaterCmd` "water" (`|MakeArray` "") "Debugger")))

(fn `OnMessageReceived`
  (params (Message :type String) (Username :type String))
  (bind _floatingtextspawner (`self.FloatingTextSpawner`)
    (:`then`
      (`/Game/KeepItAlive/Blueprints/FloatingTextSpawner.SpawnText` _floatingtextspawner (`|FormatText` "{user}: {message}" (`KismetTextLibrary.Conv_StringToText` Username) (`KismetTextLibrary.Conv_StringToText` Message))))
    (:`else`
      (bind _outactors (`GameplayStatics.GetAllActorsOfClass` "/Game/KeepItAlive/Blueprints/FloatingTextSpawner.FloatingTextSpawner_C"))
      (set `self.FloatingTextSpawner` (`|GetArrayItem` _outactors)))))

(fn `OnWaterCmd`
  (params (CommandName :type String) (CommandOptions :type "Array of String") (`Sender Username` :type String))
  (`self.ExecuteWaterCommand` CommandName CommandOptions `Sender Username`))

(fn `UserConstructionScript`)