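; FloatingTextSpawner is an actor that spawns floating text in the world around its own location.
; SpawnText creates a text actor with a fixed rotation, offset by a random amount on each axis, and sets its TextRender component to the given text.
; The SpawnVariance X and Y values act as the minimum and maximum of the random offset shared by all three axes.
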(fn `SpawnText`
  (params (Text :type Text))
  (bind (_returnvalue_x _returnvalue_y _returnvalue_z) (`KismetMathLibrary.BreakVector` (`self.K2_GetActorLocation`)))
  (bind (_spawnvariance_x _spawnvariance_y) (`KismetMathLibrary.BreakVector2D` (`self.SpawnVariance`)))
  (bind (_spawnvariance_x_2 _spawnvariance_y_2) (`KismetMathLibrary.BreakVector2D` (`self.SpawnVariance`)))
  (bind (_spawnvariance_x_3 _spawnvariance_y_3) (`KismetMathLibrary.BreakVector2D` (`self.SpawnVariance`)))
  (bind _returnvalue (`|SpawnActorFromClass` "/Game/KeepItAlive/Blueprints/FloatingText.FloatingText_C" (`KismetMathLibrary.MakeTransform` (`KismetMathLibrary.MakeVector` (+ _returnvalue_x (`KismetMathLibrary.RandomFloatInRange` _spawnvariance_x_2 _spawnvariance_y_2)) (+ _returnvalue_y (`KismetMathLibrary.RandomFloatInRange` _spawnvariance_x_3 _spawnvariance_y_3)) (+ _returnvalue_z (`KismetMathLibrary.RandomFloatInRange` _spawnvariance_x _spawnvariance_y))) (struct :`Yaw` -144.37912)) "Undefined" "OverrideRootScale" null null))
  (`TextRenderComponent.K2_SetText` (`/Game/KeepItAlive/Blueprints/FloatingText.TextRender` _returnvalue) Text))

(fn `UserConstructionScript`)